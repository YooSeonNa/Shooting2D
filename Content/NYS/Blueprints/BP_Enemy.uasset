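; Enemy actor that flies in a straight line and ends the game when it overlaps the player.
; On BeginPlay a random roll against RateToPlayer either aims and rotates it at the player's current position or keeps its forward vector.
; Tick moves it along that fixed Direction at Speed, without sweep or homing.
; Overlapping BP_Player destroys both, pauses the game and shows WBP_GameOver with cursor and UI-only input.
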(event EventBeginPlay
  (bind _returnvalue (Game|Player|GetPlayerPawn 0))
  (if (< (Math|Random|RandomIntegerinRange 0 9) (Variables|Default|GetRateToPlayer))
    (Utilities|IsValid _returnvalue
      (:Is%20Valid
        (bind _output_get (Variables|Default|SetDirection (Math|Vector|Normalize (- (Transformation|GetActorLocation _returnvalue) (Transformation|GetActorLocation)))))
        (Transformation|SetActorRotation (Math|Rotator|MakeRotfromXZ _output_get (Transformation|GetActorUpVector)))))
    (else
      (Variables|Default|SetDirection (Transformation|GetActorForwardVector)))))

(event Collision|EventActorBeginOverlap
  (params (OtherActor :type Actor%20Object%20Reference))
  (bind _returnvalue (Game|GetPlayerController 0))
  (bind _asbp_player (Utilities|Casting|CastToBP_Player OtherActor))
  (Actor|DestroyActor _asbp_player)
  (Actor|DestroyActor)
  ;[0.15 0.15 0.15 0.5] 주인공이 파괴되었으니 게임오버 처리를 하고 싶다.
  (Game|SetGamePaused true)
  (bind _returnvalue_2 (UserInterface|CreateWidget "/Game/NYS/UI/WBP_GameOver.WBP_GameOver_C"))
  (UserInterface|Viewport|AddtoViewport _returnvalue_2 0)
  ;[0.15 0.15 0.15 0.5] 게임오버가 되면 커서가 보이고  UI가 입력을 받도록 하고 싶다.
  (Variables|/Script/Engine.PlayerController|SetbShowMouseCursor _returnvalue true)
  (Input|SetInputModeUIOnly _returnvalue 0 "DoNotLock" false))

(event EventTick
  (params (DeltaSeconds :type Float%20%28single-precision%29))
  ;[0.15 0.15 0.15 0.5] Direction의 방향으로 이동한다. P = P0 +vt
  (Transformation|SetActorLocation (+ (Transformation|GetActorLocation) (* (Variables|Default|GetDirection) (Variables|Default|GetSpeed) (Utilities|Time|GetWorldDeltaSeconds))) false false))

(fn ConstructionScript)