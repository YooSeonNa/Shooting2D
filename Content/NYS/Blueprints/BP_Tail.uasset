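; BP_Tail is an actor that continuously moves toward a Target, defaulting to the player pawn when none is set at BeginPlay.
; Each Tick computes the normalized direction to the Target and passes it to Translate with Speed and world delta seconds.
; Translate offsets the location by direction, speed and delta time without sweep, so movement ignores collision and has no stopping distance.
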(event EventBeginPlay
  ;[0.15 0.15 0.15 0.5] 태어날때 Target이 설정되어 있지 않다면 플레이어를 타겟으로 설정한다.
  (Utilities|IsValid (Variables|Default|GetTarget)
    (:Is%20Not%20Valid
      (Variables|Default|SetTarget (Game|Player|GetPlayerPawn 0)))))

(event Collision|EventActorBeginOverlap
  (params (OtherActor :type Actor%20Object%20Reference)))

(event EventTick
  (params (DeltaSeconds :type Float%20%28single-precision%29))
  (CallFunction|Translate (Math|Vector|Normalize (- (Transformation|GetActorLocation (Variables|Default|GetTarget)) (Transformation|GetActorLocation))) (Variables|Default|GetSpeed) (Utilities|Time|GetWorldDeltaSeconds)))

(fn ConstructionScript)

(fn Translate
  (params (Direction :type Vector) (Speed :type Float%20%28double-precision%29) (Delta%20Second :type Float%20%28double-precision%29))
  (Transformation|SetActorLocation (+ (Transformation|GetActorLocation) (* Direction Speed Delta%20Second)) false false))