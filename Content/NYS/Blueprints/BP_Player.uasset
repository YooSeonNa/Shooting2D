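; BP_Player is the player actor of a shooter, moving in its right/up plane and firing BP_Bullet.
; BeginPlay hides the cursor and sets game-only input; the Fire press spawns a bullet at FirePosition with a blaster sound.
; Tick normalizes horizontal and vertical input into a direction for Translate, which sets location by speed and delta time without sweeping.
; An unconnected constant rightward-movement chain remains unused.
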(event EventBeginPlay
  (bind _returnvalue (Game|GetPlayerController 0))
  ;[0.15 0.15 0.15 0.5] 게임이 시작되면 커서가 안보이고 화면이 입력을 받도록 하고 싶다.
  (Variables|/Script/Engine.PlayerController|SetbShowMouseCursor _returnvalue false)
  (Input|SetInputModeGameOnly _returnvalue false))

(event Collision|EventActorBeginOverlap
  (params (OtherActor :type Actor%20Object%20Reference)))

(event EventTick
  (params (DeltaSeconds :type Float%20%28single-precision%29))
  (CallFunction|Translate (Math|Vector|Normalize (+ (* (Transformation|GetActorRightVector) (Input|AxisValues|GetHorizontal)) (* (Transformation|GetActorUpVector) (Input|AxisValues|GetVertical)))) (Variables|Default|GetSpeed) DeltaSeconds))

(event Input|ActionEvents|InputActionFire
  (params (Key :type Key%20Structure :default "None"))
  ;[0.15 0.15 0.15 0.5] 발사키를 눌렀을때 총알을 FirePosition에서 스폰하자
  (:Pressed
    (Game|SpawnActorfromClass "/Game/NYS/Blueprints/BP_Bullet.BP_Bullet_C" (Transformation|GetWorldTransform (Variables|Default|GetFirePosition)) "Undefined" "MultiplyWithRoot" 0 0)
    (Audio|PlaySound2D "/Game/NYS/Sound/star-wars-blaster.star-wars-blaster" 1.0 1.0 0.0 0 0)))

(fn ConstructionScript)

(fn Translate
  (params (Direction :type Vector) (Speed :type Float%20%28double-precision%29) (Delta%20Second :type Float%20%28double-precision%29))
  (Transformation|SetActorLocation (+ (Transformation|GetActorLocation) (* Direction Speed Delta%20Second)) false false))