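; Game mode that puts up the main UI and tracks the current score and a persistent high score.
; BeginPlay loads the "Score" save slot as BP_ScoreData, or creates a new save object, to seed HighScore.
; AddCurrentScore accumulates points, and UpdateHighScore saves CurrentScore to the slot only when it beats the record.
; The game-over widget creation in the event graph is disconnected and never runs.
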(event EventBeginPlay
  (bind _returnvalue (UserInterface|CreateWidget "/Game/NYS/UI/WBP_MainUI.WBP_MainUI_C"))
  (UserInterface|Viewport|AddtoViewport _returnvalue 0)
  (bind _returnvalue_2 (SaveGame|DoesSaveGameExist "Score"))
  (if _returnvalue_2
    (bind _returnvalue_3 (SaveGame|LoadGamefromSlot "Score"))
    (bind _asbp_score_data (Utilities|Casting|CastToBP_ScoreData _returnvalue_3))
    (bind _output_get (Variables|Default|SetSave%20Ref _asbp_score_data))
    (Variables|Default|SetHighScore (Variables|/Game/NYS/SaveData/BP_ScoreData.BP_ScoreData_C|GetBestScore _output_get))
    (else
      (bind _returnvalue_4 (SaveGame|CreateSaveGameObject "/Game/NYS/SaveData/BP_ScoreData.BP_ScoreData_C"))
      (bind _output_get_2 (Variables|Default|SetSave%20Ref _returnvalue_4))
      (Variables|Default|SetHighScore (Variables|/Game/NYS/SaveData/BP_ScoreData.BP_ScoreData_C|GetBestScore _output_get_2)))))

(event EventTick
  (params (DeltaSeconds :type Float%20%28single-precision%29)))

(fn ConstructionScript)

(fn AddCurrentScore
  (params (Point :type Integer))
  (Variables|Default|SetCurrentScore (+ Point (Variables|Default|GetCurrentScore))))

(fn UpdateHighScore
  (bind _currentscore (Variables|Default|GetCurrentScore))
  (bind _save_ref (Variables|Default|GetSave%20Ref))
  (if (> _currentscore (Variables|Default|GetHighScore))
    (bind _output_get (Variables|Default|SetHighScore _currentscore))
    (Variables|/Game/NYS/SaveData/BP_ScoreData.BP_ScoreData_C|SetBestScore _save_ref _output_get)
    (SaveGame|SaveGametoSlot _save_ref "Score")))